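; Interactive record player actor with an openable dust cover, power toggle, volume control and mute.
; Montages animate the cover and power changes, with turning on or off allowed only while open.
; Turning on starts a delayed random track from MusicDiscoMap at the actor's location, and Tick spins the vinyl while on.
; Volume input adjusts the clamped audio multiplier and rotates the knob, while AlterWBPDisco swaps open/close widgets to match the cover state.
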(event `self.ReceiveBeginPlay`
  (`self.TurnDiscoOff`))

(event `TurnDiscoOpen`
  (`|PlayMontage` (`self.RecordPlayer`) "/Game/Art/Animations/AM_RPDustCover_Opening.AM_RPDustCover_Opening"
    (:`then`
      (set `self.DiscoIsOpen` true))))

(event `TurnDiscoOn`
  (if (`self.DiscoIsOpen`)
    (`|PlayMontage` (`self.RecordPlayer`) "/Game/Art/Animations/AM_VinilPlayer_TurningOn.AM_VinilPlayer_TurningOn"
      (:`then`
        (set `self.DiscoIsOn` true)
        (`KismetSystemLibrary.K2_SetTimer` null "PlayMusicDisco" 2.5)))))

(event `TurnDiscoClose`
  (`|PlayMontage` (`self.RecordPlayer`) "/Game/Art/Animations/AM_RPDustCover_Closing.AM_RPDustCover_Closing"
    (:`then`
      (set `self.DiscoIsOpen` false))))

(event `TurnDiscoOff`
  (if (`self.DiscoIsOpen`)
    (if (`self.DiscoIsOn`)
      (`|PlayMontage` (`self.RecordPlayer`) "/Game/Art/Animations/AM_VinilPlayer_TurningOff.AM_VinilPlayer_TurningOff"
        (:`then`
          (set `self.DiscoIsOn` false)
          (`self.StopMusicDisco`)
          (set `self.SoundMuteIsOn` true))))))

(event `ToggleDiscoOpenClose`
  (if (`self.DiscoIsOpen`)
    (`self.TurnDiscoClose`)
    (else
      (`self.TurnDiscoOpen`))))

(event `ToggleDiscoOnOff`
  (if (`self.DiscoIsOn`)
    (`self.TurnDiscoOff`)
    (else
      (`self.TurnDiscoOn`))))

(event `AlterWBPDisco`
  (`WidgetLayoutLibrary.RemoveAllWidgets`)
  (if (`self.DiscoIsOpen`)
    (bind _returnvalue (`|CreateWidget` "/Game/Blueprints/Widgets/WBP_CloseTocaDiscos.WBP_CloseTocaDiscos_C"))
    (`UserWidget.AddToViewport` _returnvalue 0)
    (else
      (bind _returnvalue_2 (`|CreateWidget` "/Game/Blueprints/Widgets/WBP_OpenTocaDiscos.WBP_OpenTocaDiscos_C"))
      (`UserWidget.AddToViewport` _returnvalue_2 0))))

(event `ChangeVolumeDisco`
  (params (`Action Value` :type "Float (double-precision)"))
  (`self.ChangeVolumeDiscordPlayer` `Action Value`))

(event `self.ReceiveTick`
  (params (DeltaSeconds :type "Float (single-precision)"))
  (if (`self.DiscoIsOn`)
    (`SceneComponent.K2_AddRelativeRotation` (`self.Vinil`) (`KismetMathLibrary.MakeRotator` 0.0 0.0 1.0) false false)))

(event `ToggleMute`
  (if (`self.SoundMuteIsOn`)
    (bind _audiocomponentdisco (`self.AudioComponentDisco`)
      (:`then`
        (`AudioComponent.SetVolumeMultiplier` _audiocomponentdisco (`self.CurrentVolume`))
        (set `self.SoundMuteIsOn` false))
      (:`else`))
    (else
      (bind _audiocomponentdisco_2 (`self.AudioComponentDisco`)
        (:`then`
          (`AudioComponent.SetVolumeMultiplier` _audiocomponentdisco_2 0.001)
          (set `self.SoundMuteIsOn` true))
        (:`else`)))))

(fn `ChangeVolumeDiscordPlayer`
  (params (`Action Value` :type "Float (double-precision)"))
  (if (`self.DiscoIsOn`)
    (bind _output_get (set `self.CurrentVolume` (`KismetMathLibrary.FClamp` (+ (`self.CurrentVolume`) (* 0.1 `Action Value`)) 0.001 1.5)))
    (if (!= _output_get (`self.LastVolume`))
      (set `self.LastVolume` (`self.CurrentVolume`))
      (`SceneComponent.K2_AddRelativeRotation` (`self.VolumeSpin`) (`KismetMathLibrary.MakeRotator` (* -2.0 `Action Value`)) false false)
      (bind _audiocomponentdisco (`self.AudioComponentDisco`)
        (:`then`
          (`AudioComponent.SetVolumeMultiplier` _audiocomponentdisco (`self.CurrentVolume`)))
        (:`else`)))))

(fn `PlayMusicDisco`
  (bind _returnvalue (`GameplayStatics.SpawnSoundAtLocation` (`KismetArrayLibrary.Array_Random` (`self.MusicDiscoMap`)) (`self.K2_GetActorLocation`) (struct) (`self.CurrentVolume`) 1.0 0.0 null null))
  (set `self.AudioComponentDisco` _returnvalue))

(fn `StopMusicDisco`
  (bind _audiocomponentdisco (`self.AudioComponentDisco`)
    (:`then`
      (`AudioComponent.Stop` _audiocomponentdisco))
    (:`else`)))

(fn `UserConstructionScript`)