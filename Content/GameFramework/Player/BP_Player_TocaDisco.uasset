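; Player Blueprint for looking around and operating a record player (BP_RecordPlayer), with camera zoom and an exit menu.
; A per-tick camera line trace caches the hit actor and component, whose tags gate power, lid, volume and zoom input.
; Mute also reaches the last hit actor when nothing is targeted.
; The exit menu blocks other input and enables Escape to quit; Tick re-adds the main UI widget while hitting untagged components.
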(event `self.ReceiveBeginPlay`
  (`EnhancedInputSubsystemInterface.AddMappingContext` (pcsubsystem `EnhancedInputLocalPlayerSubsystem` (`GameplayStatics.GetPlayerController` 0)) "/Game/Input/IMC_DiscoController.IMC_DiscoController" 0 (struct))
  (bind _returnvalue (`|CreateWidget` "/Game/Blueprints/Widgets/WBP_TocaDiscosInteraction_MainUI.WBP_TocaDiscosInteraction_MainUI_C"))
  (`UserWidget.AddToViewport` _returnvalue 0))

(event `self.ReceiveTick`
  (params (DeltaSeconds :type "Float (single-precision)"))
  (`self.ExecuteLineTracing`)
  (bind _hit_toca_disco_component (`self.Hit Toca Disco Component`)
    (:`then`
      (if (`ActorComponent.ComponentHasTag` _hit_toca_disco_component "TocaDisco")
        (bind _asbp_record_player (cast `/Game/Blueprints/BP_RecordPlayer` (`self.Hit Toca Disco`)))
        (`/Game/Blueprints/BP_RecordPlayer.AlterWBPDisco` _asbp_record_player)
        (else
          (bind _returnvalue (`|CreateWidget` "/Game/Blueprints/Widgets/WBP_TocaDiscosInteraction_MainUI.WBP_TocaDiscosInteraction_MainUI_C"))
          (`UserWidget.AddToViewport` _returnvalue 0))))
    (:`else`)))

(event `EnhancedInput|/Game/Input/IA_CameraMovement`
  (params (ActionValue :type "Vector2D Structure") (ElapsedSeconds :type "Float (double-precision)") (TriggeredSeconds :type "Float (double-precision)") (InputAction :type "InputAction Object Reference" :default "/Game/Input/IA_CameraMovement.IA_CameraMovement"))
  (:`Triggered`
    (if (not (`self.MenuExitIsOn`))
      (`self.AddControllerYawInput` ActionValue_X)
      (`self.AddControllerPitchInput` (* ActionValue_Y -1.0)))))

(event `EnhancedInput|/Game/Input/IA_PlayerZoom`
  (params (ActionValue :type "Float (double-precision)") (ElapsedSeconds :type "Float (double-precision)") (TriggeredSeconds :type "Float (double-precision)") (InputAction :type "InputAction Object Reference" :default "/Game/Input/IA_PlayerZoom.IA_PlayerZoom"))
  (:`Triggered`
    (if (not (`self.MenuExitIsOn`))
      (`self.ExecuteZoomPlayer` ActionValue))))

(event `EnhancedInput|/Game/Input/IA_TurnOnDisco`
  (params (ActionValue :type Boolean) (ElapsedSeconds :type "Float (double-precision)") (TriggeredSeconds :type "Float (double-precision)") (InputAction :type "InputAction Object Reference" :default "/Game/Input/IA_TurnOnDisco.IA_TurnOnDisco"))
  (:`Completed`
    (if (not (`self.MenuExitIsOn`))
      (bind _hit_toca_disco_component (`self.Hit Toca Disco Component`)
        (:`then`
          (if (`ActorComponent.ComponentHasTag` _hit_toca_disco_component "TocaDisco")
            (bind _asbp_record_player (cast `/Game/Blueprints/BP_RecordPlayer` (`self.Hit Toca Disco`)))
            (`/Game/Blueprints/BP_RecordPlayer.ToggleDiscoOnOff` _asbp_record_player)))
        (:`else`)))))

(event `EnhancedInput|/Game/Input/IA_OpenDisco`
  (params (ActionValue :type Boolean) (ElapsedSeconds :type "Float (double-precision)") (TriggeredSeconds :type "Float (double-precision)") (InputAction :type "InputAction Object Reference" :default "/Game/Input/IA_OpenDisco.IA_OpenDisco"))
  (:`Completed`
    (if (not (`self.MenuExitIsOn`))
      (bind _hit_toca_disco_component (`self.Hit Toca Disco Component`)
        (:`then`
          (if (`ActorComponent.ComponentHasTag` _hit_toca_disco_component "TocaDisco")
            (bind _asbp_record_player (cast `/Game/Blueprints/BP_RecordPlayer` (`self.Hit Toca Disco`)))
            (`/Game/Blueprints/BP_RecordPlayer.ToggleDiscoOpenClose` _asbp_record_player)))
        (:`else`)))))

(event `EnhancedInput|/Game/Input/IA_AlterVolume`
  (params (ActionValue :type "Float (double-precision)") (ElapsedSeconds :type "Float (double-precision)") (TriggeredSeconds :type "Float (double-precision)") (InputAction :type "InputAction Object Reference" :default "/Game/Input/IA_AlterVolume.IA_AlterVolume"))
  (:`Triggered`
    (if (not (`self.MenuExitIsOn`))
      (bind _hit_toca_disco_component (`self.Hit Toca Disco Component`)
        (:`then`
          (if (`ActorComponent.ComponentHasTag` _hit_toca_disco_component "BoxVolumeSpin")
            (bind _asbp_record_player (cast `/Game/Blueprints/BP_RecordPlayer` (`self.Hit Toca Disco`)))
            (`/Game/Blueprints/BP_RecordPlayer.ChangeVolumeDisco` _asbp_record_player ActionValue)))
        (:`else`)))))

(event `EnhancedInput|/Game/Input/IA_MuteMusic`
  (params (ActionValue :type Boolean) (ElapsedSeconds :type "Float (double-precision)") (TriggeredSeconds :type "Float (double-precision)") (InputAction :type "InputAction Object Reference" :default "/Game/Input/IA_MuteMusic.IA_MuteMusic"))
  (:`Completed`
    (if (not (`self.MenuExitIsOn`))
      (bind _hit_toca_disco_component (`self.Hit Toca Disco Component`)
        (:`then`
          (if (`ActorComponent.ComponentHasTag` _hit_toca_disco_component "TocaDisco")
            (bind _asbp_record_player (cast `/Game/Blueprints/BP_RecordPlayer` (`self.Hit Toca Disco`) :!label _label))
            (`/Game/Blueprints/BP_RecordPlayer.ToggleMute` _asbp_record_player)))
        (:`else`
          (goto _label))))))

(event `EnhancedInput|/Game/Input/IA_MenuExit`
  (params (ActionValue :type Boolean) (ElapsedSeconds :type "Float (double-precision)") (TriggeredSeconds :type "Float (double-precision)") (InputAction :type "InputAction Object Reference" :default "/Game/Input/IA_MenuExit.IA_MenuExit"))
  (:`Completed`
    (`self.ToggleMenuExit`)))

(event `ToggleMenuExit`
  (`WidgetLayoutLibrary.RemoveAllWidgets`)
  (if (`self.MenuExitIsOn`)
    (bind _returnvalue (`|CreateWidget` "/Game/Blueprints/Widgets/WBP_TocaDiscosInteraction_MainUI.WBP_TocaDiscosInteraction_MainUI_C"))
    (`UserWidget.AddToViewport` _returnvalue 0)
    (set `self.MenuExitIsOn` false)
    (else
      (bind _returnvalue_2 (`|CreateWidget` "/Game/Blueprints/Widgets/WBP_MenuExit.WBP_MenuExit_C"))
      (`UserWidget.AddToViewport` _returnvalue_2 0)
      (set `self.MenuExitIsOn` true))))

(event `Key|Escape`
  (params (Key :type "Key Structure"))
  (:`Released`
    (if (`self.MenuExitIsOn`)
      (`KismetSystemLibrary.QuitGame` null "Quit"))))

(fn `ExecuteLineTracing`
  (bind _camera (`self.Camera`))
  (bind _returnvalue (`SceneComponent.K2_GetComponentLocation` _camera))
  (bind (_outhit _returnvalue_2) (`KismetSystemLibrary.LineTraceSingle` :`Start` _returnvalue :`End` (+ _returnvalue (* (`SceneComponent.GetForwardVector` _camera) 200.0)) :`TraceChannel` "TraceTypeQuery1" :`DrawDebugType` "ForOneFrame"))
  (if _returnvalue_2
    (set `self.Hit Toca Disco` (`.HitActor` (`GameplayStatics.BreakHitResult` _outhit)))
    (set `self.Hit Toca Disco Component` (`.HitComponent` (`GameplayStatics.BreakHitResult` _outhit)))
    (else
      (set `self.Hit Toca Disco Component` null))))

(fn `ExecuteZoomPlayer`
  (params (ZoomAmount :type "Float (double-precision)"))
  (bind _hit_toca_disco_component (`self.Hit Toca Disco Component`)
    (:`then`
      (if (not (`ActorComponent.ComponentHasTag` _hit_toca_disco_component "BoxVolumeSpin"))
        (bind _output_get (set `self.ZoomAmount` ZoomAmount :!label _label))
        (`CameraComponent.SetFieldOfView` (`self.Camera`) (`KismetMathLibrary.FClamp` (- (`CameraComponent.FieldOfView` (`self.Camera`)) (* _output_get (`self.SpeedZoom`))) 20.0 90.0))))
    (:`else`
      (goto _label))))

(fn `UserConstructionScript`)